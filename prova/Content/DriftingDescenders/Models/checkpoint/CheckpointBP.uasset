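; Checkpoint actor for a timed car run that saves the player's respawn point and can double as the finish line.
; On first exit it stores the UiManager timer, updates the car's respawn transform, plays audio, turns its lights green and shows a popup.
; RestartTimer writes the stored time back to the timer UI.
; When flagged as last, entering it ends the car's run and score, disables death and opens the FinishMenu.
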(event OnComponentEndOverlap(collisionBox)
  (params (OverlappedComponent :type Primitive%20Component%20Object%20Reference) (OtherActor :type Actor%20Object%20Reference) (OtherComp :type Primitive%20Component%20Object%20Reference) (OtherBodyIndex :type Integer))
  (if (== OtherActor (Game|Player|GetPlayerPawn 0))
    (if (Variables|Default|GetalreadyUsed?)
      (bind _ascar_ray_bp (Utilities|Casting|CastTocarRayBP (Game|Player|GetPlayerPawn 0)))
      (Variables|/Game/VehicleArcade/carRayBP.carRayBP_C|SetlastCheckpoint _ascar_ray_bp self)
      (else
        (Utilities|FlowControl|Sequence
          (:then_0
            (CallFunction|GetTime))
          (:then_1
            (Audio|Components|Audio|Play (Variables|Default|GetcheckpointAudio) 0.0))
          (:then_2
            (bind _ascar_ray_bp_2 (Utilities|Casting|CastTocarRayBP (Game|Player|GetPlayerPawn 0)))
            (Utilities|FlowControl|Sequence
              (:then_0
                (Variables|/Game/VehicleArcade/carRayBP.carRayBP_C|SetlastCheckpointLocation _ascar_ray_bp_2 (Transformation|GetWorldLocation (Variables|Default|GetSpawnCar))))
              (:then_1
                (Variables|/Game/VehicleArcade/carRayBP.carRayBP_C|SetlastCheckpoint _ascar_ray_bp_2 self))
              (:then_2
                (Variables|Default|SetalreadyUsed? true))
              (:then_3
                (Variables|/Game/VehicleArcade/carRayBP.carRayBP_C|SetlastCheckpointRotation _ascar_ray_bp_2 (Transformation|GetActorRotation self)))
              (:then_4
                (bind _returnvalue (UserInterface|CreateWidget "/Game/UI/checkPointReachedUI.checkPointReachedUI_C"))
                (UserInterface|Viewport|AddtoViewport _returnvalue 0))))
          (:then_3
            (for _array_element (Actor|GetComponentsByClass "/Script/Engine.PointLightComponent")
              (Rendering|Components|Light|SetLightColor _array_element (Utilities|Struct|MakeLinearColor 0.0 1.0 0.0 1.0) true))))))))

(event OnComponentBeginOverlap(collisionBox)
  (params (OverlappedComponent :type Primitive%20Component%20Object%20Reference) (OtherActor :type Actor%20Object%20Reference) (OtherComp :type Primitive%20Component%20Object%20Reference) (OtherBodyIndex :type Integer) (bFromSweep :type Boolean) (SweepResult :type Hit%20Result%20Structure%20%28by%20ref%29))
  (if (== OtherActor (Game|Player|GetPlayerPawn 0))
    (if (Variables|Default|GetlastCheckpoint?)
      (CallFunction|GetTime)
      (CallFunction|OnEndRun)
      (bind _returnvalue (UserInterface|CreateWidget "/Game/UI/finishMenu.finishMenu_C" (Game|GetPlayerController 0)))
      (bind _output_get (Variables|Default|SetfinishMenu _returnvalue))
      (UserInterface|Viewport|AddtoViewport _output_get 0))))

(event Custom|RestartTimer
  (bind _outactors (Actor|GetAllActorsOfClass "/Game/UI/UiManager.UiManager_C"))
  (for _array_element _outactors
    (Utilities|FlowControl|Sequence
      (:then_0
        (Variables|/Game/UI/Widget_Timer.Widget_Timer_C|SetsecondsElapsed (Variables|/Game/UI/UiManager.UiManager_C|GetTimerUI _array_element) (Variables|Default|Getseconds)))
      (:then_1
        (Variables|/Game/UI/Widget_Timer.Widget_Timer_C|SetminutesElapsed (Variables|/Game/UI/UiManager.UiManager_C|GetTimerUI _array_element) (Variables|Default|Getminutes)))
      (:then_2
        (Variables|/Game/UI/Widget_Timer.Widget_Timer_C|SetmilisecondsElapsed (Variables|/Game/UI/UiManager.UiManager_C|GetTimerUI _array_element) (Variables|Default|Getmiliseconds))))))

(fn ConstructionScript)

(fn GetTime
  (bind _returnvalue (Actor|GetActorOfClass "/Game/UI/UiManager.UiManager_C"))
  (Utilities|FlowControl|Sequence
    (:then_0
      (Variables|Default|Setseconds (Variables|/Game/UI/Widget_Timer.Widget_Timer_C|GetsecondsElapsed (Variables|/Game/UI/UiManager.UiManager_C|GetTimerUI _returnvalue))))
    (:then_1
      (Variables|Default|Setminutes (Variables|/Game/UI/Widget_Timer.Widget_Timer_C|GetminutesElapsed (Variables|/Game/UI/UiManager.UiManager_C|GetTimerUI _returnvalue))))
    (:then_2
      (Variables|Default|Setmiliseconds (Variables|/Game/UI/Widget_Timer.Widget_Timer_C|GetmilisecondsElapsed (Variables|/Game/UI/UiManager.UiManager_C|GetTimerUI _returnvalue))))))

(fn OnEndRun
  (bind _ascar_ray_bp (Utilities|Casting|CastTocarRayBP (Game|Player|GetPlayerPawn 0)))
  (Default|EndCombo (Variables|/Game/VehicleArcade/carRayBP.carRayBP_C|GetScoreManager _ascar_ray_bp))
  (Default|CallOnEndRunTime _ascar_ray_bp (Variables|Default|Getminutes) (Variables|Default|Getseconds) (Variables|Default|Getmiliseconds))
  (Variables|/Game/VehicleArcade/carRayBP.carRayBP_C|SetcanDie _ascar_ray_bp false)
  (Default|CallOnEndRunGeneric _ascar_ray_bp)
  (Default|EndRun (Variables|/Game/VehicleArcade/carRayBP.carRayBP_C|GetScoreManager _ascar_ray_bp)))