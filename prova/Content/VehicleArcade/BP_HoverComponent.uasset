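; Raycast suspension component for an arcade vehicle (carRayBP) that pushes the car body up from the ground and positions its child wheel mesh.
; Each tick it traces along its local down axis, setting CanRun by comparing hit distance to the vehicle's CheckDistance.
; On a hit within range, it moves the wheel toward the contact point and applies a spring force with clamped damping to the vehicle root at the component's location.
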(event EventBeginPlay
  (bind _ascar_ray_bp (Utilities|Casting|CastTocarRayBP (Components|GetOwner)))
  (bind _output_get (Variables|Default|SetParentVehicle _ascar_ray_bp)))

(event EventTick
  (params (DeltaSeconds :type Float%20%28single-precision%29))
  (bind _returnvalue (Transformation|GetWorldLocation))
  (bind _returnvalue_2 (Components|GetChildComponent 0))
  (bind _asstatic_mesh_component (Utilities|Casting|CastToStaticMeshComponent _returnvalue_2))
  (bind _returnvalue_3 (Transformation|GetWorldLocation _asstatic_mesh_component))
  (Utilities|IsValid (Variables|Default|GetParentVehicle)
    (:Is%20Valid
      (bind (_outhit _returnvalue_4) (Collision|LineTraceByChannel _returnvalue (- _returnvalue (/ (* (Math|Vector|GetUpVector) (Variables|Default|GetSpringCarDistance)) 1.0)) "TraceTypeQuery1" false 0 "None"))
      (bind _output_get (Variables|Default|SetOut%20Hit _outhit))
      (Variables|Default|SetDistanceFromFloor (.Distance (Collision|BreakHitResult _output_get)))
      (if (<= (.Distance (Collision|BreakHitResult _output_get)) (Variables|/Game/VehicleArcade/carRayBP.carRayBP_C|GetCheckDistance (stale EventBeginPlay _output_get)))
        (Variables|Default|SetcanRun true)
        (if _returnvalue_4
          (if (<= (Math|Vector|VectorLength (- (.Location (Collision|BreakHitResult _output_get)) _returnvalue_3)) 1e+01)
            (Variables|Default|SetnewWheelLocation (+ (.Location (Collision|BreakHitResult _output_get)) (* (* (Math|Vector|GetUpVector self) -1) (Variables|Default|GetspringDistance))))
            (else
              (Variables|Default|SetnewWheelLocation (+ _returnvalue_3 (* (Math|Vector|Normalize (- (.Location (Collision|BreakHitResult _output_get)) _returnvalue_3)) (* DeltaSeconds (Variables|Default|GetWheelRecolocationSpeed)))))))
          (Transformation|SetWorldLocation _asstatic_mesh_component (Variables|Default|GetnewWheelLocation) false false)
          (bind _output_get_2 (Variables|Default|SetSpringDelta (- (Variables|Default|GetSpringCarDistance) (.Distance (Collision|BreakHitResult _output_get)))))
          (Class|PrimitiveComponent|AddForceatLocation (.AsPrimitive%20Component (Utilities|Casting|CastToPrimitiveComponent (Variables|/Script/Engine.Actor|GetRootComponent (Variables|Default|GetParentVehicle)))) (* (Math|Vector|GetUpVector) (+ (* (/ (Math|Float|Clamp(Float) (- _output_get_2 (Variables|Default|GetPreviousSpringDelta)) (* (Variables|Default|GetClamp) -1.0) (Variables|Default|GetClamp)) (Utilities|Time|GetWorldDeltaSeconds)) (Variables|Default|GetDampingCoeficient)) (* _output_get_2 (Variables|Default|GetSpringCoeficient)))) (Transformation|GetWorldLocation) "None")
          (Variables|Default|SetPreviousSpringDelta (Variables|Default|GetSpringDelta)))
        (else
          (Variables|Default|SetcanRun false))))))